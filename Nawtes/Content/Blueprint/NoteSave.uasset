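; NoteSave holds a list of notes for saving and provides helpers to edit and format them.
; DeleteFromSave removes a note from NotesList, and ParseNote builds a single string from section, separator and content.
; SaveSection is an empty stub, and Debug prints entries to screen, though its loop has no array connected.
; No function here writes to disk or adds notes.
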(fn `Debug`
  ;[1 0.92 0.05788] Just for debug, calm down
  (`KismetSystemLibrary.PrintString` null "printing results" true true (struct :`R` 1.0 :`G` 0.014152 :`B` 0.123819 :`A` 1.0) 10.0)
  (for _array_element _
    (`KismetSystemLibrary.PrintString` null (`KismetTextLibrary.Conv_TextToString` _array_element) true true (struct :`R` 1.0 :`G` 0.222369 :`B` 0.883104 :`A` 1.0) 10.0)))

(fn `DeleteFromSave`
  (params (NoteToDelete :type String))
  (`KismetArrayLibrary.Array_RemoveItem` (`self.NotesList`) NoteToDelete))

(fn `ParseNote`
  (params (Content :type Text) (Section :type String))
  (returns (ParsedNote :type String))
  (return (`KismetStringLibrary.Concat_StrStr` Section (`KismetStringLibrary.Concat_StrStr` (`self.Separator`) (`KismetTextLibrary.Conv_TextToString` Content)))))

(fn `SaveSection`
  (params (NewSection :type String)))